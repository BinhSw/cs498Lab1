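; BP_Projectile is a projectile actor that flies in a straight line along world X and removes itself on contact or timeout.
; Tick moves it with a swept world offset scaled by ProjectileSpeed and delta time, with no movement component involved.
; The construction script records the creation time, which Tick checks to destroy it after three seconds.
; Cylinder overlaps also destroy it, except with components whose object name is TriggerZone.
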(event OnComponentBeginOverlap(Cylinder)
  (params (OverlappedComponent :type Primitive%20Component%20Object%20Reference) (OtherActor :type Actor%20Object%20Reference) (OtherComp :type Primitive%20Component%20Object%20Reference) (OtherBodyIndex :type Integer) (bFromSweep :type Boolean) (SweepResult :type Hit%20Result%20Structure%20%28by%20ref%29))
  (if (not (Utilities|Name|Equal(Name) (Utilities|String|StringToName (Utilities|GetObjectName OtherComp)) "TriggerZone"))
    (Actor|DestroyActor)))

(event EventBeginPlay)

(event EventTick
  (params (DeltaSeconds :type Float%20%28single-precision%29))
  (if (> (- (Utilities|Time|GetGameTimeinSeconds) (Variables|Default|GetCreateTime)) 3.0)
    (Actor|DestroyActor)
    (else
      (Transformation|AddActorWorldOffset (Math|Vector|MakeVector (* (Variables|Default|GetProjectileSpeed) DeltaSeconds) 0.0 0.0) true))))

(fn ConstructionScript
  (Variables|Default|SetCreateTime (Utilities|Time|GetTimeSeconds)))